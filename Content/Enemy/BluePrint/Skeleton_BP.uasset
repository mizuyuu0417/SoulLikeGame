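; Skeleton enemy character that runs Skeleton_BT, attacks with a sword and dies when its health runs out.
; On BeginPlay it spawns a HeroSword_BP on its hand socket, passes it to TraceComponent and links itself to its health bar widget.
; Damage updates the bar and plays a hit montage, or on death stops the AI once.
; Attack plays a random montage and stores its length; Clear empties the trace ignore list.
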(event Custom|Attack
  (bind _returnvalue (Animation|PlayAnimMontage (.OutItem (Utilities|Array|Random (Variables|Default|Getattackanimations))) 1.0 "None"))
  (Variables|Default|SetattackLength _returnvalue))

(event Custom|Clear
  (Utilities|Array|Clear (Variables|/Game/Equipment/TraceComponent.TraceComponent_C|Getactortoignore (Variables|Default|GetTraceComponent))))

(event EventBeginPlay
  ;[1 1 1] Ai System
  (AI|RunBehaviorTree (AI|GetAIController self) "/Game/Enemy/BehaviourTree/Skeleton_BT.Skeleton_BT")
  (bind _returnvalue (Game|SpawnActorfromClass "/Game/Equipment/HeroSword_BP.HeroSword_BP_C" (Transformation|GetSocketTransform (Variables|Character|GetMesh) "sword" "RTS_World") "Undefined" 0 0))
  (bind _output_get (Variables|Default|Setsword_enemy_ref _returnvalue))
  (Transformation|AttachComponentToComponent _output_get (Variables|Character|GetMesh) "sword" "SnapToTarget" "SnapToTarget" "SnapToTarget" true)
  (Variables|/Game/Equipment/TraceComponent.TraceComponent_C|Setsword_ref (Variables|Default|GetTraceComponent) (Variables|Default|Getsword_enemy_ref))
  (bind _asskeleton_health_bar_wbp (Utilities|Casting|CastToSkeletonHealthBar_WBP (UserInterface|GetWidget (Variables|Default|GetHealthBar))))
  (bind _output_get_2 (Variables|Default|SetAs%20Skeleton%20Health%20Bar_ref _asskeleton_health_bar_wbp))
  (Variables|/Game/Enemy/BluePrint/SkeletonHealthBar_WBP.SkeletonHealthBar_WBP_C|SetSkeleton_ref _output_get_2 self))

(event Collision|EventActorBeginOverlap
  (params (OtherActor :type Actor%20Object%20Reference)))

(event EventTick
  (params (DeltaSeconds :type Float%20%28single-precision%29)))

(event Game|Damage|EventAnyDamage
  (params (Damage :type Float%20%28single-precision%29) (DamageType :type Damage%20Type%20Object%20Reference) (InstigatedBy :type Controller%20Object%20Reference) (DamageCauser :type Actor%20Object%20Reference))
  (bind _output_get (Variables|Default|SetHealth (- (Variables|Default|GetHealth) Damage)))
  (if (<= _output_get 0.0)
    (Rendering|SetVisibility (Variables|Default|GetHealthBar) false false)
    (Utilities|FlowControl|DoOnce false
      (:Completed
        (AI|Logic|StopLogic (Variables|/Script/AIModule.AIController|GetBrainComponent (AI|GetAIController self)) "")
        (Animation|PlayAnimMontage "/Game/Enemy/Animation/SkeleDeath_Montage.SkeleDeath_Montage" 1.0 "None")))
    (else
      (Rendering|SetVisibility (Variables|Default|GetHealthBar) true false)
      (Default|UpadteHealthBar (Variables|Default|GetAs%20Skeleton%20Health%20Bar_ref))
      (Animation|PlayAnimMontage "/Game/Enemy/Animation/Skele_Hit_Montage.Skele_Hit_Montage" 1.0 "None"))))

(fn ConstructionScript)